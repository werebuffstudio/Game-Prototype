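; AC_StateCharacter is a character state component that is mostly a stub for item pickup and throw handling.
; On BeginPlay it calls SetRef, which casts player character 0 to BP_ThirdPersonCharacter and caches the reference.
; The Spawnitempickup and Throw_item events are empty.
; Disconnected leftover nodes hold unfinished logic for actor destroy and spawn, attachment to an "item" socket and a State change.
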(event Custom|Throw%20_item
  (params (Mesh :type Mesh%20Component%20Object%20Reference)))

(event Custom|Spawn%20item%20pickup
  (params (RowName :type Name)))

(event Custom|set%20Ref
  (bind _asbp_third_person_character (Utilities|Casting|CastToBP_ThirdPersonCharacter (Game|GetPlayerCharacter 0)))
  (Variables|Default|SetAs%20BP%20Third%20Person%20Character_0 _asbp_third_person_character))

(event EventBeginPlay
  (CallFunction|SetRef))

(event EventTick
  (params (DeltaSeconds :type Float%20%28single-precision%29)))