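; BP_itemPickup is a pickup item actor whose mesh comes from the DT_State_Item data table.
; The setitem event applies the row's mesh to Sphere, while BeginPlay looks up NameItem without using the result.
; FunctionPickup fires once, asking the character's ACStateCharacter to spawn a hardcoded "Cup" item.
; FunctionThow enables gravity and collision on Sphere but turns physics simulation off.
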(event Custom|set%20item
  (params (RowName :type Name))
  (bind _returnvalue (Utilities|GetDataTableRow "/Game/DATA/DataTable/DT_State_Item.DT_State_Item" RowName)
    (:then
      (Components|StaticMesh|SetStaticMesh (Variables|Default|GetSphere) (.Actor (Utilities|Struct|BreakF_State_Item _returnvalue))))))

(event EventBeginPlay
  (bind _returnvalue (Utilities|GetDataTableRow "/Game/DATA/DataTable/DT_State_Item.DT_State_Item" (Variables|Default|GetName_item))))

(event Collision|EventActorBeginOverlap
  (params (OtherActor :type Actor%20Object%20Reference)))

(event EventTick
  (params (DeltaSeconds :type Float%20%28single-precision%29)))

(fn ConstructionScript)

(fn FunctionPickup
  (params (character :type BP%20Player%20Object%20Reference))
  (Utilities|FlowControl|DoOnce false
    (:Completed
      (Default|SpawnItemPickup (Variables|/Game/ThirdPerson/Blueprints/BP_Player.BP_Player_C|GetAC_StateCharacter character) "Cup")
      (return false))))

(fn FunctionThow
  (bind _sphere (Variables|Default|GetSphere))
  (Physics|SetSimulatePhysics _sphere false)
  (Physics|SetEnableGravity _sphere true)
  (Collision|SetCollisionEnabled _sphere "QueryAndPhysics")
  (return false))