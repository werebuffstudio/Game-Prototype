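; Thrown item actor that launches as a projectile and then becomes a loose physics object.
; Its setitem event looks up a row in DT_State_Item to set the Sphere component's static mesh and store the item name.
; On BeginPlay, short delays deactivate ProjectileMovement, then switch Sphere to simulated physics with collision and gravity.
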(event Custom|set%20item
  (params (RowName :type Name))
  (bind _returnvalue (Utilities|GetDataTableRow "/Game/DATA/DataTable/DT_State_Item.DT_State_Item" RowName)
    (:then
      (Components|StaticMesh|SetStaticMesh (Variables|Default|GetSphere) (.Actor (Utilities|Struct|BreakF_State_Item _returnvalue)))
      (Variables|Default|SetName (.Name (Utilities|Struct|BreakF_State_Item _returnvalue))))))

(event EventBeginPlay
  (bind _sphere (Variables|Default|GetSphere))
  (Utilities|FlowControl|Delay 0.5)
  (Components|Activation|Deactivate (Variables|Default|GetProjectileMovement))
  (Utilities|FlowControl|Delay 0.2)
  (Physics|SetSimulatePhysics _sphere true)
  (Collision|SetCollisionEnabled _sphere "QueryAndPhysics")
  (Physics|SetEnableGravity (Variables|Default|GetSphere) true))

(event Collision|EventActorBeginOverlap
  (params (OtherActor :type Actor%20Object%20Reference)))

(event EventTick
  (params (DeltaSeconds :type Float%20%28single-precision%29)))

(fn ConstructionScript)